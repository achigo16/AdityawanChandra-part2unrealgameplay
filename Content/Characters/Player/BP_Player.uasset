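; BP_Player is the player character Blueprint, providing movement and a sword attack through Enhanced Input.
; BeginPlay adds the game's mapping context, and the move action drives movement relative to control rotation with pitch zeroed.
; The attack action plays a sword combo montage and sets IsAttack to block movement input.
; A DoOnce gate prevents re-triggering until a delay equal to the montage's returned duration clears the flag.
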(event Input|EnhancedActionEvents|EnhancedInputActionIA_Move
  (params (ActionValue :type Vector%202D%20Structure) (ElapsedSeconds :type Float%20%28double-precision%29) (TriggeredSeconds :type Float%20%28double-precision%29) (InputAction :type Input%20Action%20Object%20Reference :default "/Game/Characters/Player/Input/IA_Move.IA_Move"))
  (bind _returnvalue (Pawn|GetControlRotation :!class /Script/Engine.Pawn))
  (bind _returnvalue_2 (Pawn|GetControlRotation :!class /Script/Engine.Pawn))
  (:Triggered
    (if (not (Variables|Default|GetIsAttack))
      (Pawn|Input|AddMovementInput (Math|Vector|GetRightVector (Math|Rotator|MakeRotator (.roll _returnvalue) 0.0 (.yaw _returnvalue))) (.x ActionValue) false)
      (Pawn|Input|AddMovementInput (Math|Vector|GetForwardVector (Math|Rotator|MakeRotator (.roll _returnvalue_2) 0.0 (.yaw _returnvalue_2))) (.y ActionValue) false))))

(event Input|EnhancedActionEvents|EnhancedInputActionIA_Attack
  (params (ActionValue :type Boolean) (ElapsedSeconds :type Float%20%28double-precision%29) (TriggeredSeconds :type Float%20%28double-precision%29) (InputAction :type Input%20Action%20Object%20Reference :default "/Game/Characters/Player/Input/IA_Attack.IA_Attack"))
  (:Triggered
    (Utilities|FlowControl|DoOnce false :!label _label
      (:Completed
        (Variables|Default|SetIsAttack true)
        (bind _returnvalue (Animation|PlayAnimMontage "/Game/Characters/Player/Animations/Kriss_Model_Anim_Armature_M_Armature_M_Attack_Sword_Combo_01_Montage.Kriss_Model_Anim_Armature_M_Armature_M_Attack_Sword_Combo_01_Montage" 1.0 "None"))
        (Utilities|FlowControl|Delay _returnvalue)
        (Variables|Default|SetIsAttack false)
        (goto _label Reset)))))

(event EventBeginPlay
  (bind _asplayer_controller (Utilities|Casting|CastToPlayerController (Pawn|GetController)))
  (Utilities|IsValid (PlayerController|LocalPlayerSubsystems|GetEnhancedInputLocalPlayerSubsystem _asplayer_controller)
    (:Is%20Valid
      (Input|AddMappingContext (PlayerController|LocalPlayerSubsystems|GetEnhancedInputLocalPlayerSubsystem _asplayer_controller) "/Game/Characters/Player/Input/IMC_MyGame.IMC_MyGame" 0 "(bIgnoreAllPressedKeysUntilRelease=True,bForceImmediately=False)"))))

(fn ConstructionScript)